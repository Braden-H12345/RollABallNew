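; Pickup that boosts the player's ball by multiplying its max angular velocity by 500 on overlap.
; A MultiGate's first output plays a coin sound, spawns a particle burst and destroys the actor.
; Its second output, needing another overlap, waits five seconds then assigns the velocity to itself, so nothing here reverts the boost.
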(event OnComponentBeginOverlap(Collision)
  (params (OverlappedComponent :type Primitive%20Component%20Object%20Reference) (OtherActor :type Actor%20Object%20Reference) (OtherComp :type Primitive%20Component%20Object%20Reference) (OtherBodyIndex :type Integer) (bFromSweep :type Boolean) (SweepResult :type Hit%20Result%20Structure%20%28by%20ref%29))
  (bind _returnvalue (Transformation|GetActorLocation))
  (if (== OtherActor (Game|Player|GetPlayerPawn 0))
    (bind _asball_pawn (Utilities|Casting|CastToBallPawn (Game|Player|GetPlayerPawn 0)))
    (Variables|/Game/_Game/BallGame/BallPawn.BallPawn_C|SetMaxAngularVelocity _asball_pawn (* (Variables|/Game/_Game/BallGame/BallPawn.BallPawn_C|GetMaxAngularVelocity _asball_pawn) 5e+02))
    (Utilities|FlowControl|MultiGate false false -1
      (:Out%200
        (Audio|PlaySoundatLocation "/Game/_Game/Audio/coinPickup_cue.coinPickup_cue" _returnvalue "0, 0, 0" 1.0 1.0 0.0 0 0 0 0)
        (Niagara|SpawnSystematLocation "/Game/_Game/Particles/PS_GenericBurst.PS_GenericBurst" _returnvalue)
        (Actor|DestroyActor))
      (:Out%201
        (Utilities|FlowControl|Delay 5.0)
        (Variables|/Game/_Game/BallGame/BallPawn.BallPawn_C|SetMaxAngularVelocity _asball_pawn (Variables|/Game/_Game/BallGame/BallPawn.BallPawn_C|GetMaxAngularVelocity _asball_pawn))))))

(fn ConstructionScript)